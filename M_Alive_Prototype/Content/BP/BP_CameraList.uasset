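; BP_CameraList is a camera actor that switches between preset distances, taking over the first player's view on BeginPlay.
; Number keys 1–4 ease the Camera component to relative offsets with half-second MoveComponentTo moves.
; OnChangeCamera selects presets by index, sharing the key moves, except that index 3 uses key 4's farthest offset, leaving key 3's middle offset keyboard-only.
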(event Custom|OnChangeCamera
  (params (CameraIndex :type String))
  (bind _camera (Variables|Default|GetCamera))
  (switch int (Math|Conversions|ToInteger(Byte) CameraIndex)
    (:1
      (Components|MoveComponentTo _camera "0, 0, 0" "0, 0, 0" true true 0.5 false))
    (:2
      (Components|MoveComponentTo _camera "-150.000000, 0,-8.000000" "0, 0, 0" true true 0.5 false))
    (:3
      (Components|MoveComponentTo _camera "-800.000000, 0,-60.000000" "0, 0, 0" true true 0.5 false :!label _label))
    (:4
      (goto _label))))

(event EventBeginPlay
  (Game|Player|SetViewTargetwithBlend (Game|GetPlayerController 0) (Components|GetOwner (Variables|Default|GetCamera)) 0.0 "VTBlend_EaseInOut" 0.0 true))

(event Input|KeyboardEvents|4
  (params (Key :type Key%20Structure :default "None"))
  (:Pressed
    (Components|MoveComponentTo (Variables|Default|GetCamera) "-800.000000, 0,-60.000000" "0, 0, 0" true true 0.5 false)))

(event Input|KeyboardEvents|1
  (params (Key :type Key%20Structure :default "None"))
  (:Pressed
    (Components|MoveComponentTo (Variables|Default|GetCamera) "0, 0, 0" "0, 0, 0" true true 0.5 false)))

(event Input|KeyboardEvents|2
  (params (Key :type Key%20Structure :default "None"))
  (:Pressed
    (Components|MoveComponentTo (Variables|Default|GetCamera) "-150.000000, 0,-8.000000" "0, 0, 0" true true 0.5 false)))

(event Input|KeyboardEvents|3
  (params (Key :type Key%20Structure :default "None"))
  (:Pressed
    (Components|MoveComponentTo (Variables|Default|GetCamera) "-300.000000, 0,-20.000000" "0, 0, 0" true true 0.5 false)))

(fn ConstructionScript)