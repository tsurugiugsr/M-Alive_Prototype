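; Test actor for a talking MetaHuman virtual assistant, with a toggleable UI and keys cycling hair and clothes.
; Holding backslash records the mic; release streams PCM chunks over WebSocket to speech-to-text and prints parsed words.
; Tick feeds UI sliders to the face post-process AnimBP and can play 30 fps morph frames through BP_MH_Talk.
; TTS requests are built but never sent; lip-data loading is disconnected and emotion updates are empty loops.
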(event Custom|EventEmotinChange
  ;[1 1 1] Comment
  (CallFunction|UpdateEmotion))

(event Custom|自定义事件_0
  (params (bSucceed :type Boolean))
  (bind _returnvalue (Math|DateTime|Now))
  (if bSucceed
    (Development|PrintString (Utilities|String|Append (Utilities|String|Append "C:\\Output\\wav_" (Utilities|String|ToString(Integer) (Class|KismetMathLibrary|GetYear _returnvalue)) "-" (Utilities|String|ToString(Integer) (Class|KismetMathLibrary|GetMonth _returnvalue)) "-" (Utilities|String|ToString(Integer) (Class|KismetMathLibrary|GetDay _returnvalue)) "-" (Utilities|String|ToString(Integer) (Class|KismetMathLibrary|GetHour _returnvalue)) "-" (Utilities|String|ToString(Integer) (Class|KismetMathLibrary|GetMinute _returnvalue)) "-" (Utilities|String|ToString(Integer) (Class|KismetMathLibrary|GetSecond _returnvalue)) ".wav") "：存储成功"))
    (else
      (Development|PrintString "文件存储失败" true true "(R=1.000000,G=0.000000,B=0.000000,A=1.000000)"))))

(event Custom|OnVpaTalk
  (params (NewParam :type String))
  ;[1 1 1] 处理页面发过来的对话信息
)

(event Custom|OnChangeHair
  (params (HairName :type String))
  ;[1 1 1] OnChangeHair
  ;[1 1 1] Key Change Hair
  (switch int (Math|Integer|%(Integer) (Variables|Default|GetHairIndex) 3)
    (:0
      (Class|GroomComponent|SetGroomAsset (Variables|Default|Gettoufa))
      (Class|GroomComponent|SetBindingAsset (Variables|Default|Gettoufa)))
    (:1
      (Class|GroomComponent|SetGroomAsset (Variables|Default|Gettoufa))
      (Class|GroomComponent|SetBindingAsset (Variables|Default|Gettoufa)))
    (:2
      (Class|GroomComponent|SetGroomAsset (Variables|Default|Gettoufa))
      (Class|GroomComponent|SetBindingAsset (Variables|Default|Gettoufa))))
  (Variables|Default|SetHairIndex (+ (Variables|Default|GetHairIndex) 1)))

(event Custom|OnChangeClothes
  (params (ClothesName :type String))
  (bind _yifu (Variables|Default|Getyifu))
  (bind _yifu_2 (Variables|Default|Getyifu))
  (bind _yifu_3 (Variables|Default|Getyifu))
  (bind _yifu_4 (Variables|Default|Getyifu))
  ;[1 1 1] OnChangeClothes
  (switch int (Math|Integer|%(Integer) (Variables|Default|GetClothesIndex) 3)
    (:0
      (Components|SkinnedMesh|SetSkinnedAssetandUpdate _yifu_3 0 true)
      (Rendering|Material|SetMaterial _yifu 0 0)
      (Rendering|Material|SetMaterial _yifu_4 1 0)
      (Rendering|Material|SetMaterial _yifu_2 2 0))
    (:1
      (Components|SkinnedMesh|SetSkinnedAssetandUpdate _yifu_3 0 true)
      (Rendering|Material|SetMaterial _yifu 0 0)
      (Rendering|Material|SetMaterial _yifu_4 1 0)
      (Rendering|Material|SetMaterial _yifu_2 2 0))
    (:2
      (Components|SkinnedMesh|SetSkinnedAssetandUpdate _yifu_3 0 true)
      (Rendering|Material|SetMaterial _yifu 0 0)
      (Rendering|Material|SetMaterial _yifu_4 1 0)
      (Rendering|Material|SetMaterial _yifu_2 2 0)))
  (Variables|Default|SetClothesIndex (+ (Variables|Default|GetClothesIndex) 1)))

(event Custom|EventButtonTalk
  (bind _mainui (Variables|Default|GetMainUI))
  (bind _mainui_2 (Variables|Default|GetMainUI))
  (bind _checkbox_tts_ms (Variables|/Game/UI/MainUI-Prototype.MainUI-Prototype_C|GetCheckBox_TTS_MS _mainui))
  (bind _textbox_talk (Variables|/Game/UI/MainUI-Prototype.MainUI-Prototype_C|GetTextBox_Talk _mainui_2))
  (bind _returnvalue (Class|CheckBox|GetCheckedState _checkbox_tts_ms))
  (bind _returnvalue_2 (Class|EditableTextBox|GetText _textbox_talk))
  (bind _returnvalue_3 (Utilities|String|ToString(Text) _returnvalue_2))
  (bind _returnvalue_4 (Utilities|String|EnumtoString _returnvalue))
  ;[1 1 1] Comment
  (if (or (Utilities|Enum|Equal(Enum) _returnvalue_4 "Checked") (Utilities|Enum|Equal(Enum) _returnvalue_4 "已勾选"))
    (Variables|Default|SetStrTts "ms")
    (else
      (Variables|Default|SetStrTts "aispeech")))
  (Variables|Default|SetrequestUrl (Utilities|String|Append "http://" (Utilities|String|ToString(Text) (Class|EditableTextBox|GetText (Variables|/Game/UI/MainUI-Prototype.MainUI-Prototype_C|GetTextBox_URL (Variables|Default|GetMainUI)))) "/audio2bs"))
  (Variables|Default|SetrequestJson (Utilities|String|Append "{\"content\": \"" _returnvalue_3 "\", \"emotion\": 1, \"amplitude\": 1 ,\"tts_type\": \"" (Variables|Default|GetStrTts) "\"}"))
  (Development|PrintString (Variables|Default|GetrequestUrl) true true "(R=0.000000,G=0.660000,B=1.000000,A=1.000000)" 1e+01)
  (Variables|Default|Setcontent _returnvalue_3)
  (Development|PrintString "1111"))

(event EventBeginPlay
  ;[1 1 1] Comment
  (bind _returnvalue (UserInterface|CreateWidget "/Game/UI/MainUI-Prototype.MainUI-Prototype_C"))
  (bind _output_get (Variables|Default|SetMainUI _returnvalue))
  (Widget|SetVisibility _output_get "Hidden")
  (UserInterface|Viewport|AddtoViewport (Variables|Default|GetMainUI) 0)
  (EventDispatchers|BindEventtoEventDispatcherEmotionChange (Variables|Default|GetMainUI) (delegate Custom|EventEmotinChange))
  (EventDispatchers|BindEventtoEventDispatcherTalk (Variables|Default|GetMainUI) (delegate Custom|EventButtonTalk))
  (bind _asface_post_process_anim_bp (Utilities|Casting|CastTo (Class|SkeletalMeshComponent|GetPostProcessInstance (Variables|Default|GetMH))))
  (Variables|Default|SetAs%20Face%20Post%20Process%20Anim%20BP _asface_post_process_anim_bp))

(event EventTick
  (params (DeltaSeconds :type Float%20%28single-precision%29))
  (bind _mainui (Variables|Default|GetMainUI))
  ;[1 1 1] Tick
  (Variables|Default|SetDelta%20Seconds DeltaSeconds)
  (Utilities|FlowControl|Sequence
    (:then_0
      (if (== (Variables|Default|GetnState) 1)
        (CallFunction|PlayLipAnimation (Variables|Default|GetDelta%20Seconds))))
    (:then_1
      (CallFunction|PlayIdel (Variables|Default|GetDelta%20Seconds))
      (Variables|Default|Set_FaceControl (Variables|Default|GetAs%20Face%20Post%20Process%20Anim%20BP) (Utilities|Array|MakeArray (Class|Slider|GetValue (Variables|/Game/UI/MainUI-Prototype.MainUI-Prototype_C|GetSlider_1 _mainui)) (Class|Slider|GetValue (Variables|/Game/UI/MainUI-Prototype.MainUI-Prototype_C|GetSlider_2 _mainui)) (Class|Slider|GetValue (Variables|/Game/UI/MainUI-Prototype.MainUI-Prototype_C|GetSlider_3 _mainui)) (Class|Slider|GetValue (Variables|/Game/UI/MainUI-Prototype.MainUI-Prototype_C|GetSlider_4 _mainui)) (Class|Slider|GetValue (Variables|/Game/UI/MainUI-Prototype.MainUI-Prototype_C|GetSlider_5 _mainui)) (Class|Slider|GetValue (Variables|/Game/UI/MainUI-Prototype.MainUI-Prototype_C|GetSlider_6 _mainui)))))))

(event Input|KeyboardEvents|F9
  (params (Key :type Key%20Structure :default "None"))
  (bind _returnvalue (Game|GetPlayerController 0))
  (bind _mainui (Variables|Default|GetMainUI))
  ;[1 1 1] 开关UI
  (:Pressed
    (Utilities|FlowControl|FlipFlop
      (:A
        (Variables|/Script/Engine.PlayerController|SetbShowMouseCursor _returnvalue true)
        (Widget|SetVisibility _mainui "Visible"))
      (:B
        (Variables|/Script/Engine.PlayerController|SetbShowMouseCursor _returnvalue false)
        (Widget|SetVisibility _mainui "Hidden")))))

(event Input|KeyboardEvents|3
  (params (Key :type Key%20Structure :default "None"))
  (bind _newvar_0 (Variables|Default|GetNewVar_0))
  (:Pressed
    (while (< _newvar_0 100)
      (Development|PrintString (Utilities|String|ToString(Integer) _newvar_0))
      (Math|Integer|IncrementInt _newvar_0
        (:%20%20
          (Utilities|FlowControl|Delay 0.05))))))

(event Input|KeyboardEvents|R
  (params (Key :type Key%20Structure :default "None"))
  (bind _mainui (Variables|Default|GetMainUI))
  (bind _mainui_2 (Variables|Default|GetMainUI))
  (bind _checkbox_tts_ms (Variables|/Game/UI/MainUI-Prototype.MainUI-Prototype_C|GetCheckBox_TTS_MS _mainui))
  (bind _textbox_talk (Variables|/Game/UI/MainUI-Prototype.MainUI-Prototype_C|GetTextBox_Talk _mainui_2))
  (bind _returnvalue (Class|CheckBox|GetCheckedState _checkbox_tts_ms))
  (bind _returnvalue_2 (Class|EditableTextBox|GetText _textbox_talk))
  (bind _returnvalue_3 (Utilities|String|ToString(Text) _returnvalue_2))
  (bind _returnvalue_4 (Utilities|String|EnumtoString _returnvalue))
  (:Pressed
    (if (or (Utilities|Enum|Equal(Enum) _returnvalue_4 "Checked") (Utilities|Enum|Equal(Enum) _returnvalue_4 "已勾选"))
      (Variables|Default|SetStrTts "ms")
      (else
        (Variables|Default|SetStrTts "aispeech")))
    (Variables|Default|SetrequestUrl (Utilities|String|Append "http://" (Utilities|String|ToString(Text) (Class|EditableTextBox|GetText (Variables|/Game/UI/MainUI-Prototype.MainUI-Prototype_C|GetTextBox_URL (Variables|Default|GetMainUI)))) "/audio2bs"))
    (Variables|Default|SetrequestJson (Utilities|String|Append "{\"content\": \"" _returnvalue_3 "\", \"emotion\": 1, \"amplitude\": 1 ,\"tts_type\": \"" (Variables|Default|GetStrTts) "\"}"))
    (Development|PrintString (Variables|Default|GetrequestUrl) true true "(R=0.000000,G=0.660000,B=1.000000,A=1.000000)" 1e+01)
    (Variables|Default|Setcontent _returnvalue_3)
    (Development|PrintString "1111")))

(event Input|KeyboardEvents|0
  (params (Key :type Key%20Structure :default "None"))
  ;[1 1 1] Key Change Hair
  (:Pressed
    (switch int (Math|Integer|%(Integer) (Variables|Default|GetHairIndex) 3)
      (:0
        (Class|GroomComponent|SetGroomAsset (Variables|Default|Gettoufa))
        (Class|GroomComponent|SetBindingAsset (Variables|Default|Gettoufa)))
      (:1
        (Class|GroomComponent|SetGroomAsset (Variables|Default|Gettoufa))
        (Class|GroomComponent|SetBindingAsset (Variables|Default|Gettoufa)))
      (:2
        (Class|GroomComponent|SetGroomAsset (Variables|Default|Gettoufa))
        (Class|GroomComponent|SetBindingAsset (Variables|Default|Gettoufa))))
    (Variables|Default|SetHairIndex (+ (Variables|Default|GetHairIndex) 1))))

(event Input|KeyboardEvents|9
  (params (Key :type Key%20Structure :default "None"))
  (bind _yifu (Variables|Default|Getyifu))
  (bind _yifu_2 (Variables|Default|Getyifu))
  (bind _yifu_3 (Variables|Default|Getyifu))
  (bind _yifu_4 (Variables|Default|Getyifu))
  (:Pressed
    (switch int (Math|Integer|%(Integer) (Variables|Default|GetClothesIndex) 3)
      (:0
        (Components|SkinnedMesh|SetSkinnedAssetandUpdate _yifu_3 0 true)
        (Rendering|Material|SetMaterial _yifu 0 0)
        (Rendering|Material|SetMaterial _yifu_4 1 0)
        (Rendering|Material|SetMaterial _yifu_2 2 0))
      (:1
        (Components|SkinnedMesh|SetSkinnedAssetandUpdate _yifu_3 0 true)
        (Rendering|Material|SetMaterial _yifu 0 0)
        (Rendering|Material|SetMaterial _yifu_4 1 0)
        (Rendering|Material|SetMaterial _yifu_2 2 0))
      (:2
        (Components|SkinnedMesh|SetSkinnedAssetandUpdate _yifu_3 0 true)
        (Rendering|Material|SetMaterial _yifu 0 0)
        (Rendering|Material|SetMaterial _yifu_4 1 0)
        (Rendering|Material|SetMaterial _yifu_2 2 0)))
    (Variables|Default|SetClothesIndex (+ (Variables|Default|GetClothesIndex) 1))))

(event Input|KeyboardEvents|Backslash
  (params (Key :type Key%20Structure :default "None"))
  (bind _audiocapture (Variables|Default|GetAudioCapture))
  (:Pressed
    (Development|PrintString "R On")
    (CameraShake|Start _audiocapture)
    (Class|AudioMixerBlueprintLibrary|StartRecordingOutput 0.0 "/Game/Touya/AudioInputAnalysis.AudioInputAnalysis"))
  (:Released
    (Development|PrintString "R Off")
    (Audio|Components|Audio|Stop _audiocapture)
    (bind _returnvalue (Class|AudioMixerBlueprintLibrary|StopRecordingOutput "SoundWave" "" "" "/Game/Touya/AudioInputAnalysis.AudioInputAnalysis" 0))
    (bind _request (CallFunction|Speech2TextInitial "a73d2cf6" "46b0adaafd93920cbb3d0d12a4338498"))
    (Development|PrintString _request)
    (bind (_result _result_2) (|AsyncWebSocket (Utilities|Struct|Make 0 _request))
      (:then
        (Variables|Default|SetWSResult _result))
      (:OnConnected
        (bind _returnvalue_2 (CallFunction|Speech2TextChannelByebye (CallFunction|GetSoundWavePCMData _returnvalue)))
        (Variables|Default|SetaudioSend _returnvalue_2)
        (Utilities|Array|Resize (Variables|Default|GetPCMChunk) 1280)
        (Variables|Default|SetPCMChunksIndex 0)
        (while (> (Utilities|Array|Length (Variables|Default|GetaudioSend)) (* (Variables|Default|GetPCMChunksIndex) 1280))
          (Variables|Default|SetPCMBytesIndex 0)
          (while (< (Variables|Default|GetPCMBytesIndex) 1280)
            (if (>= (+ (Variables|Default|GetPCMBytesIndex) (* (Variables|Default|GetPCMChunksIndex) 1280)) (Utilities|Array|Length (Variables|Default|GetaudioSend)))
              (Utilities|Array|SetArrayElem (Variables|Default|GetPCMChunk) (Variables|Default|GetPCMBytesIndex) 0)
              (else
                (Utilities|Array|SetArrayElem (Variables|Default|GetPCMChunk) (Variables|Default|GetPCMBytesIndex) (Utilities|Array|Get(acopy) (Variables|Default|GetaudioSend) (+ (Variables|Default|GetPCMBytesIndex) (* (Variables|Default|GetPCMChunksIndex) 1280))))))
            (Math|Integer|IncrementInt (Variables|Default|GetPCMBytesIndex)))
          (CallFunction|SendBytes (Variables|Default|GetWSResult) (Variables|Default|GetPCMChunk) true)
          (Math|Integer|IncrementInt (Variables|Default|GetPCMChunksIndex)))
        (bind _returnvalue_3 (CallFunction|UStringtoBytes (Variables|Default|Getend_tag)))
        (CallFunction|SendBytes (Variables|Default|GetWSResult) _returnvalue_3 true))
      (:OnTextMessage
        (Variables|Default|SetSpeech2TextResult (.TextMessage (Utilities|Struct|Break _result_2))))
      (:OnClosed
        (Development|PrintString (Variables|Default|GetSpeech2TextResult))
        (Variables|Default|SetMicInResult "")
        (while (.ReturnValue (Utilities|String|Split (Variables|Default|GetSpeech2TextResult) "\"w\\\":\\\""))
          (Variables|Default|SetMicInResult (Utilities|String|Append (Variables|Default|GetMicInResult) (.LeftS (Utilities|String|Split (.RightS (Utilities|String|Split (Variables|Default|GetSpeech2TextResult) "\"w\\\":\\\"")) "\\"))))
          (Variables|Default|SetSpeech2TextResult (.RightS (Utilities|String|Split (Variables|Default|GetSpeech2TextResult) "\"w\\\":\\\""))))
        (Development|PrintString (Variables|Default|GetMicInResult))))))

(fn ConstructionScript)

(fn UpdateEmotion
  (bind _struct_bs_face_ctrl (Variables|Default|GetStruct%20Bs%20Face%20Ctrl))
  (bind (_bs_name_surprised _surprised _issurprised _bs_name_shock _shock _isshock _bs_name_frown _frown _isfrown _bs_name_flirting _flirting _isflirting _bs_name_angry _angry _isangry _bs_name_smileopenfullface _smileopenfullface _issmileopenfullface _bs_name_smilefullface _smilefullface _issmilefullface _bs_name_afraid) (Utilities|Struct|BreakStruct_BsFaceCtrl _struct_bs_face_ctrl))
  (Utilities|FlowControl|Sequence
    (:then_0
      (for _array_element _bs_name_surprised
        _))
    (:then_1
      (for _array_element_2 _bs_name_shock
        _))
    (:then_2
      (for _array_element_3 _bs_name_frown
        _))
    (:then_3
      (for _array_element_4 _bs_name_flirting
        _))
    (:then_4
      (for _array_element_5 _bs_name_angry
        _))
    (:then_5
      (for _array_element_6 _bs_name_smileopenfullface
        _))
    (:then_6
      (for _array_element_7 _bs_name_smilefullface
        _))
    (:then_7
      (for _array_element_8 _bs_name_afraid
        _))))

(fn PlayLipAnimation
  (params (DeltaTime :type Float%20%28double-precision%29))
  (bind _output_get (Variables|Default|SetCurFpsTime (+ DeltaTime (Variables|Default|GetCurFpsTime))))
  (if (!= (Math|Float|Truncate (/ _output_get 0.033333)) (Variables|Default|GetCurAnimationTimes))
    (Variables|Default|SetCurAnimationTimes (Math|Float|Truncate (/ _output_get 0.033333)))
    (if (> (Variables|Default|GetMaxAnimationTimes) (Variables|Default|GetCurAnimationTimes))
      (Utilities|Map|Clear (Variables|Default|GetTempMap))
      (for (_array_element _array_index) (Variables|Default|GetBsKeyList)
        (Utilities|Map|Add (Variables|Default|GetTempMap) _array_element (Utilities|Array|Get(acopy) (Variables|Default|GetMorphArray) (+ _array_index (* (Variables|Default|GetCurAnimationTimes) (Utilities|Array|Length (Variables|Default|GetBsKeyList)))))))
      (bind _asbp_mh_talk (Utilities|Casting|CastToBP_MH_Talk (Components|SkeletalMesh|GetAnimInstance (Variables|Default|GetMH))))
      (Variables|/Game/BP/AnimationBP/BP_MH_Talk.BP_MH_Talk_C|SetCurBsList _asbp_mh_talk (Variables|Default|GetTempMap))
      (else
        (Variables|Default|SetnState 0)))))

(fn ProtobuftoLipData
  (params (JsonString :type Array%20of%20Bytes))
  (Utilities|Array|Clear (Variables|Default|GetMorphArray))
  (Utilities|Array|Clear (Variables|Default|GetBsKeyList))
  (Utilities|Array|Clear (Variables|Default|GetwavData)))

(fn KeyNametoDazName
  (params (NewParam :type Array%20of%20Names))
  (for _array_element NewParam
    (switch name _array_element ; Live name
      (:Default
        (Utilities|Array|Add (Variables|Default|GetBsDazNameList) "null"))
      (:jawForward
        ;[1 1 1] 控制口型
        (Utilities|Array|Add (Variables|Default|GetBsDazNameList) "Genesis8_1Female__facs_jnt_JawForward"))
      (:jawLeft
        (Utilities|Array|Add (Variables|Default|GetBsDazNameList) "Genesis8_1Female__facs_jnt_JawLeft"))
      (:jawRight
        (Utilities|Array|Add (Variables|Default|GetBsDazNameList) "Genesis8_1Female__facs_jnt_JawRight"))
      (:jawOpen
        (Utilities|Array|Add (Variables|Default|GetBsDazNameList) "Genesis8_1Female__facs_jnt_JawOpen"))
      (:mouthClose
        (Utilities|Array|Add (Variables|Default|GetBsDazNameList) "Genesis8_1Female__facs_bs_MouthClose_div2"))
      (:mouthLeft
        (Utilities|Array|Add (Variables|Default|GetBsDazNameList) "Genesis8_1Female__facs_bs_MouthLeft_div2"))
      (:mouthRight
        (Utilities|Array|Add (Variables|Default|GetBsDazNameList) "Genesis8_1Female__facs_bs_MouthRight_div2"))
      (:mouthSmileLeft
        (Utilities|Array|Add (Variables|Default|GetBsDazNameList) "Genesis8_1Female__facs_bs_MouthSmileLeft_div2"))
      (:mouthSmileRight
        (Utilities|Array|Add (Variables|Default|GetBsDazNameList) "Genesis8_1Female__facs_bs_MouthSmileRight_div2"))
      (:mouthDimpleLeft
        (Utilities|Array|Add (Variables|Default|GetBsDazNameList) "Genesis8_1Female__facs_bs_MouthDimpleLeft_div2"))
      (:mouthDimpleRight
        (Utilities|Array|Add (Variables|Default|GetBsDazNameList) "Genesis8_1Female__facs_bs_MouthDimpleRight_div2"))
      (:mouthStretchLeft
        (Utilities|Array|Add (Variables|Default|GetBsDazNameList) "Genesis8_1Female__facs_bs_MouthStretchLeft_div2"))
      (:mouthStretchRight
        (Utilities|Array|Add (Variables|Default|GetBsDazNameList) "Genesis8_1Female__facs_bs_MouthStretchRight_div2"))
      (:mouthShrugLower
        (Utilities|Array|Add (Variables|Default|GetBsDazNameList) "Genesis8_1Female__facs_bs_MouthShrugLower_div2"))
      (:mouthShrugUpper
        (Utilities|Array|Add (Variables|Default|GetBsDazNameList) "Genesis8_1Female__facs_bs_MouthShrugUpper_div2"))
      (:mouthPressLeft
        (Utilities|Array|Add (Variables|Default|GetBsDazNameList) "Genesis8_1Female__facs_bs_MouthPressLeft_div2"))
      (:mouthPressRight
        (Utilities|Array|Add (Variables|Default|GetBsDazNameList) "Genesis8_1Female__facs_bs_MouthPressRight_div2"))
      (:mouthLowerDownLeft
        (Utilities|Array|Add (Variables|Default|GetBsDazNameList) "Genesis8_1Female__facs_bs_MouthLowerDownLeft_div2"))
      (:mouthLowerDownRight
        (Utilities|Array|Add (Variables|Default|GetBsDazNameList) "Genesis8_1Female__facs_bs_MouthLowerDownRight_div2"))
      (:mouthUpperUpLeft
        (Utilities|Array|Add (Variables|Default|GetBsDazNameList) "Genesis8_1Female__facs_bs_MouthUpperUpLeft_div2"))
      (:mouthUpperUpRight
        (Utilities|Array|Add (Variables|Default|GetBsDazNameList) "Genesis8_1Female__facs_bs_MouthUpperUpRight_div2"))
      (:mouthFunnel
        (Utilities|Array|Add (Variables|Default|GetBsDazNameList) "Genesis8_1Female__facs_bs_MouthFunnel_div2"))
      (:mouthPucker
        (Utilities|Array|Add (Variables|Default|GetBsDazNameList) "Genesis8_1Female__facs_bs_MouthPucker_div2"))
      (:mouthFrownLeft
        (Utilities|Array|Add (Variables|Default|GetBsDazNameList) "Genesis8_1Female__facs_bs_MouthFrownLeft_div2"))
      (:mouthFrownRight
        (Utilities|Array|Add (Variables|Default|GetBsDazNameList) "Genesis8_1Female__facs_bs_MouthFrownRight_div2"))
      (:mouthRollLower
        (Utilities|Array|Add (Variables|Default|GetBsDazNameList) "Genesis8_1Female__facs_bs_MouthRollLower_div2"))
      (:mouthRollUpper
        (Utilities|Array|Add (Variables|Default|GetBsDazNameList) "Genesis8_1Female__facs_bs_MouthRollUpper_div2"))
      (:browdownleft
        ;[1 1 1] Comment
        (Utilities|Array|Add (Variables|Default|GetBsDazNameList) "Genesis8_1Female__facs_bs_BrowDownLeft_div2"))
      (:browupleft
        (Utilities|Array|Add (Variables|Default|GetBsDazNameList) "Genesis8_1Female__facs_ctrl_BrowUp"))
      (:browinnerup
        (Utilities|Array|Add (Variables|Default|GetBsDazNameList) "Genesis8_1Female__facs_ctrl_BrowInnerUp"))
      (:browdownright
        (Utilities|Array|Add (Variables|Default|GetBsDazNameList) "Genesis8_1Female__facs_bs_BrowDownRight_div2"))
      (:eyeblinkleft
        (Utilities|Array|Add (Variables|Default|GetBsDazNameList) "Genesis8_1Female__facs_jnt_EyeBlinkLeft"))
      (:eyewideleft
        (Utilities|Array|Add (Variables|Default|GetBsDazNameList) "Genesis8_1Female__facs_jnt_EyeWideLeft"))
      (:eyeblinkright
        (Utilities|Array|Add (Variables|Default|GetBsDazNameList) "Genesis8_1Female__facs_jnt_EyeBlinkRight"))
      (:eyewideright
        (Utilities|Array|Add (Variables|Default|GetBsDazNameList) "Genesis8_1Female__facs_jnt_EyeWideRight"))
      (:headdown
        ;[1 1 1] 控制头部
        (Utilities|Array|Add (Variables|Default|GetBsDazNameList) "headdown"))
      (:headleft
        (Utilities|Array|Add (Variables|Default|GetBsDazNameList) "headleft"))
      (:headtiltleft
        (Utilities|Array|Add (Variables|Default|GetBsDazNameList) "headtiltleft"))
      (:eyeLookUpRight
        ;[1 1 1] Comment
        (Utilities|Array|Add (Variables|Default|GetBsDazNameList) "Genesis8_1Female__facs_jnt_EyeLookUpRight"))
      (:eyeLookOutRight
        (Utilities|Array|Add (Variables|Default|GetBsDazNameList) "Genesis8_1Female__facs_bs_EyeLookOutRight_div2"))
      (:eyeLookInRight
        (Utilities|Array|Add (Variables|Default|GetBsDazNameList) "Genesis8_1Female__facs_bs_EyeLookInRight_div2"))
      (:eyeLookDownRight
        (Utilities|Array|Add (Variables|Default|GetBsDazNameList) "Genesis8_1Female__facs_jnt_EyeLookDownRight"))
      (:eyeLookUpLeft
        (Utilities|Array|Add (Variables|Default|GetBsDazNameList) "Genesis8_1Female__facs_jnt_EyeLookUpLeft"))
      (:eyeLookOutLeft
        (Utilities|Array|Add (Variables|Default|GetBsDazNameList) "Genesis8_1Female__facs_bs_EyeLookOutLeft_div2"))
      (:eyeLookInLeft
        (Utilities|Array|Add (Variables|Default|GetBsDazNameList) "Genesis8_1Female__facs_bs_EyeLookInLeft_div2"))
      (:eyeLookDownLeft
        (Utilities|Array|Add (Variables|Default|GetBsDazNameList) "Genesis8_1Female__facs_jnt_EyeLookDownLeft"))
      (:eyeSquintRight
        (Utilities|Array|Add (Variables|Default|GetBsDazNameList) "Genesis8_1Female__facs_bs_EyeSquintRight_div2"))
      (:eyeSquintLeft
        (Utilities|Array|Add (Variables|Default|GetBsDazNameList) "Genesis8_1Female__facs_bs_EyeSquintLeft_div2"))
      (:tongueOut
        ;[1 1 1] 其他
        (Utilities|Array|Add (Variables|Default|GetBsDazNameList) "Genesis8_1Female__facs_bs_TongueOut"))
      (:cheekPuff
        (Utilities|Array|Add (Variables|Default|GetBsDazNameList) "Genesis8_1Female__facs_ctrl_CheekPuff"))
      (:cheekSquintLeft
        (Utilities|Array|Add (Variables|Default|GetBsDazNameList) "Genesis8_1Female__facs_bs_CheekSquintLeft_div2"))
      (:cheekSquintRight
        (Utilities|Array|Add (Variables|Default|GetBsDazNameList) "Genesis8_1Female__facs_bs_CheekSquintRight_div2"))
      (:noseSneerRight
        (Utilities|Array|Add (Variables|Default|GetBsDazNameList) "Genesis8_1Female__facs_bs_NoseSneerRight_div2"))
      (:noseSneerLeft
        (Utilities|Array|Add (Variables|Default|GetBsDazNameList) "Genesis8_1Female__facs_bs_NoseSneerLeft_div2"))
      (:browOuterUpLeft
        (Utilities|Array|Add (Variables|Default|GetBsDazNameList) "Genesis8_1Female__facs_bs_BrowOuterUpLeft_div2"))
      (:browOuterUpRight
        (Utilities|Array|Add (Variables|Default|GetBsDazNameList) "Genesis8_1Female__facs_bs_BrowOuterUpRight_div2"))
      (:mouthUp
        (Utilities|Array|Add (Variables|Default|GetBsDazNameList) "Genesis8_1Female__facs_ctrl_MouthUpperUp")))))

(fn PlayIdel
  (params (DeltaTime :type Float%20%28double-precision%29)))

(fn AudioPCMSplit
  (params (PCMData :type Array%20of%20Bytes))
  (return 0))