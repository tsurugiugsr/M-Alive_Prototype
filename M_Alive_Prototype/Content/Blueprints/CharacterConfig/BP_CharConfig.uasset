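; BP_CharConfig is a character configurator actor that switches the displayed character and its skin on a skeletal mesh.
; ChangeCharacter loads the row named after the character index from DT_CharSelect, then applies its first skin.
; ChangeSkin sets the indexed mesh, reapplies that mesh's default materials and assigns the row's animation Blueprint.
; Tick stores the BP_Orbit_Pawn camera's world location in a variable.
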(event Custom|ChangeSkin
  (params (NewSkinIndex :type Integer))
  (bind _currentdatatablerow (Variables|Default|GetCurrentDataTableRow))
  (bind _skelmesh (Utilities|Struct|BreakCharSelect_Struct _currentdatatablerow))
  ;[1 1 1] Change skin event
  (bind _output_get (Variables|Default|SetCurrentSkinIndex NewSkinIndex))
  (if (Utilities|Array|IsValidIndex _skelmesh _output_get)
    (Utilities|IsValid (Utilities|Array|Get(acopy) _skelmesh _output_get)
      (:Is%20Valid
        (Class|SkinnedMeshComponent|SetSkeletalMesh (Variables|Default|GetSkeletalMesh) (Utilities|Array|Get(acopy) _skelmesh _output_get) true)
        (for (_array_element _array_index) (Variables|/Script/Engine.SkeletalMesh|GetMaterials (Utilities|Array|Get(acopy) _skelmesh _output_get))
          (Rendering|Material|SetMaterial (Variables|Default|GetSkeletalMesh) _array_index (.MaterialInterface (Utilities|Struct|BreakSkeletalMaterial _array_element))))
        (Class|SkeletalMeshComponent|SetAnimClass (Variables|Default|GetSkeletalMesh) (.AnimBP (Utilities|Struct|BreakCharSelect_Struct (Variables|Default|GetCurrentDataTableRow))))))
    (else
      (Development|PrintString "Error: Skin not found"))))

(event Custom|ChangeCharacter
  (params (NewCharacterIndex :type Integer))
  ;[1 1 1] Change character event
  (if (!= NewCharacterIndex (Variables|Default|GetCurrentCharacterIndex))
    (Variables|Default|SetCurrentCharacterIndex NewCharacterIndex)
    (bind _returnvalue (Utilities|GetDataTableRow "/Game/Blueprints/CharacterConfig/DT_CharSelect.DT_CharSelect" (Utilities|String|StringToName (Utilities|String|ToString(Integer) (Variables|Default|GetCurrentCharacterIndex))))
      (:then
        (Variables|Default|SetCurrentDataTableRow _returnvalue)
        (CallFunction|ChangeSkin))
      (:RowNotFound
        (Development|PrintString "Error: Char row not found on DataTable")))))

(event EventTick
  (params (DeltaSeconds :type Float%20%28single-precision%29))
  ;[1 1 1] Update the camera position each tick
  (bind _asbp_orbit_pawn (Utilities|Casting|CastToBP_Orbit_Pawn (Game|Player|GetPlayerPawn 0)))
  (Variables|Default|SetCameraWorldLocation (Transformation|GetWorldLocation (Variables|/Game/Blueprints/Pawn/BP_Orbit_Pawn.BP_Orbit_Pawn_C|GetFirstPersonCamera _asbp_orbit_pawn))))

(event EventBeginPlay
  ;[1 1 1] Set starting charcter to index 0
  (CallFunction|ChangeCharacter 1))

(fn ConstructionScript)