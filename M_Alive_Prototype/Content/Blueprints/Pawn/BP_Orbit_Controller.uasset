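; Orbit controller for a Pixel Streaming configurator that turns browser JSON messages into in-game changes.
; BeginPlay caches the orbit pawn, character config, VPA meta and camera list actors, then binds the input listener.
; OnJSONEvent routes by field name to character, skin, environment, time, zoom, camera, talk, hair or clothes changes, or runs raw console commands.
; Environment and time changes toggle streaming sublevel visibility behind timed camera fades.
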(event Custom|OnJSONEvent
  (params (Descriptor :type String))
  ;[1 1 1] Bind JSON events - This is listening for HTM/Java events from the Pixel Streaming client's web browser.
  (bind _output_get (Variables|Default|SetDescriptor Descriptor))
  (Development|PrintString _output_get)
  (if (.Success (Class|PixelStreamingInput|GetJsonStringValue (Variables|Default|GetPixelStreamingInput) (Variables|Default|GetDescriptor) "Category"))
    (CallFunction|ChangeConfigOption)
    (elif (.Success (Class|PixelStreamingInput|GetJsonStringValue (Variables|Default|GetPixelStreamingInput) (Variables|Default|GetDescriptor) "Zoom"))
      (CallFunction|ToggleZoom)
      (elif (.Success (Class|PixelStreamingInput|GetJsonStringValue (Variables|Default|GetPixelStreamingInput) (Variables|Default|GetDescriptor) "Console"))
        (Development|ExecuteConsoleCommand (.StringValue (Class|PixelStreamingInput|GetJsonStringValue (Variables|Default|GetPixelStreamingInput) (Variables|Default|GetDescriptor) "Console")) 0)
        (elif (Class|BlueprintJsonLibrary|JsonHasField (Class|BlueprintJsonLibrary|ToJsonObject(String) (Variables|Default|GetDescriptor)) "Talk")
          (Default|OnVpaTalk (Variables|Default|GetVpaMeta) (Variables|Default|GetDescriptor))
          (elif (.Success (Class|PixelStreamingInput|GetJsonStringValue (Variables|Default|GetPixelStreamingInput) (Variables|Default|GetDescriptor) "Camera"))
            (Default|OnChangeCamera (Variables|Default|GetCameraList) (.StringValue (Class|PixelStreamingInput|GetJsonStringValue (Variables|Default|GetPixelStreamingInput) (Variables|Default|GetDescriptor) "Camera")))
            (elif (.Success (Class|PixelStreamingInput|GetJsonStringValue (Variables|Default|GetPixelStreamingInput) (Variables|Default|GetDescriptor) "Hair"))
              (Default|OnChangeHair (Variables|Default|GetVpaMeta) (.StringValue (Class|PixelStreamingInput|GetJsonStringValue (Variables|Default|GetPixelStreamingInput) (Variables|Default|GetDescriptor) "Hair")))
              (elif (.Success (Class|PixelStreamingInput|GetJsonStringValue (Variables|Default|GetPixelStreamingInput) (Variables|Default|GetDescriptor) "Clothes"))
                (Default|OnChangeClothes (Variables|Default|GetVpaMeta) (.StringValue (Class|PixelStreamingInput|GetJsonStringValue (Variables|Default|GetPixelStreamingInput) (Variables|Default|GetDescriptor) "Clothes")))))))))))

(event Custom|ChangeCharacter
  (bind _pixelstreaminginput (Variables|Default|GetPixelStreamingInput))
  (bind _descriptor (Variables|Default|GetDescriptor))
  (bind _stringvalue (Class|PixelStreamingInput|GetJsonStringValue _pixelstreaminginput _descriptor "Item"))
  ;[1 1 1] Change Character
  (Development|PrintString _stringvalue true true "(R=1.000000,G=0.409627,B=0.000000,A=1.000000)" 2e+01)
  (Default|ChangeCharacter (Variables|Default|GetCharConfigRef) (Math|Conversions|ToInteger(Byte) _stringvalue)))

(event Custom|ChangeEnv
  ;[1 1 1] Change Env
  (Variables|Default|SetMapSelection (.StringValue (Class|PixelStreamingInput|GetJsonStringValue (Variables|Default|GetPixelStreamingInput) (Variables|Default|GetDescriptor) "Item")))
  (CameraFades|StartCameraFade :self (Game|GetPlayerCameraManager 0) :ToAlpha 1.0 :Duration 0.5 :bShouldFadeAudio true :bHoldWhenFinished true)
  (Utilities|FlowControl|Delay 0.7)
  (Variables|/Script/Engine.LevelStreaming|SetbShouldBeVisible (Class|GameplayStatics|GetStreamingLevel "Fortress_Base") (Utilities|Enum|Equal(Enum) (Variables|Default|GetMapSelection) "1"))
  (Variables|/Script/Engine.LevelStreaming|SetbShouldBeVisible (Class|GameplayStatics|GetStreamingLevel "Ruins_Daylight") false)
  (Variables|/Script/Engine.LevelStreaming|SetbShouldBeVisible (Class|GameplayStatics|GetStreamingLevel "Ruins_Night") false)
  (Variables|/Script/Engine.LevelStreaming|SetbShouldBeVisible (Class|GameplayStatics|GetStreamingLevel "Ruins_Base") (Utilities|Enum|Equal(Enum) (Variables|Default|GetMapSelection) "0"))
  (Variables|/Script/Engine.LevelStreaming|SetbShouldBeVisible (Class|GameplayStatics|GetStreamingLevel "Fortress_Daylight") false)
  (Variables|/Script/Engine.LevelStreaming|SetbShouldBeVisible (Class|GameplayStatics|GetStreamingLevel "Fortress_Night") false)
  (CallFunction|ChangeTime true))

(event Custom|ChangeSkin
  ;[1 1 1] Change Skin
  (Default|ChangeSkin (Variables|Default|GetCharConfigRef) (Math|Conversions|ToInteger(Byte) (.StringValue (Class|PixelStreamingInput|GetJsonStringValue (Variables|Default|GetPixelStreamingInput) (Variables|Default|GetDescriptor) "Item")))))

(event Custom|ChangeTime
  (params (BypassHTML :type Boolean))
  ;[1 1 1] Change Time of Day
  (if BypassHTML
    _
    (else
      (Variables|Default|SetCurrentTime (.StringValue (Class|PixelStreamingInput|GetJsonStringValue (Variables|Default|GetPixelStreamingInput) (Variables|Default|GetDescriptor) "Item")))
      (CameraFades|StartCameraFade :self (Game|GetPlayerCameraManager 0) :ToAlpha 1.0 :Duration 0.5 :bShouldFadeAudio true :bHoldWhenFinished true)
      (Utilities|FlowControl|Delay 0.7)))
  (switch string (Variables|Default|GetMapSelection)
    (:0
      (switch string (Variables|Default|GetCurrentTime)
        (:0
          (Variables|/Script/Engine.LevelStreaming|SetbShouldBeVisible (Class|GameplayStatics|GetStreamingLevel "Ruins_Daylight") true)
          (Variables|/Script/Engine.LevelStreaming|SetbShouldBeVisible (Class|GameplayStatics|GetStreamingLevel "Ruins_Night") false))
        (:1
          (Variables|/Script/Engine.LevelStreaming|SetbShouldBeVisible (Class|GameplayStatics|GetStreamingLevel "Ruins_Daylight") false)
          (Variables|/Script/Engine.LevelStreaming|SetbShouldBeVisible (Class|GameplayStatics|GetStreamingLevel "Ruins_Night") true))))
    (:1
      (switch string (Variables|Default|GetCurrentTime)
        (:0
          (Variables|/Script/Engine.LevelStreaming|SetbShouldBeVisible (Class|GameplayStatics|GetStreamingLevel "Fortress_Daylight") true)
          (Variables|/Script/Engine.LevelStreaming|SetbShouldBeVisible (Class|GameplayStatics|GetStreamingLevel "Fortress_Night") false))
        (:1
          (Variables|/Script/Engine.LevelStreaming|SetbShouldBeVisible (Class|GameplayStatics|GetStreamingLevel "Fortress_Daylight") false)
          (Variables|/Script/Engine.LevelStreaming|SetbShouldBeVisible (Class|GameplayStatics|GetStreamingLevel "Fortress_Night") true)))))
  (Utilities|FlowControl|Delay 0.5)
  (CameraFades|StartCameraFade :self (Game|GetPlayerCameraManager 0) :FromAlpha 1.0 :Duration 0.5 :bShouldFadeAudio true))

(event Custom|ToggleZoom
  (bind _playerpawn (Variables|Default|GetPlayerPawn))
  ;[1 1 1] JSON Event: Toggle Zoom
  (switch string (.StringValue (Class|PixelStreamingInput|GetJsonStringValue (Variables|Default|GetPixelStreamingInput) (Variables|Default|GetDescriptor) "Zoom"))
    (:1
      (Utilities|FlowControl|FlipFlop
        (:A
          (Variables|/Game/Blueprints/Pawn/BP_Orbit_Pawn.BP_Orbit_Pawn_C|SetTargetZoom _playerpawn 1.2e+02))
        (:B
          (Variables|/Game/Blueprints/Pawn/BP_Orbit_Pawn.BP_Orbit_Pawn_C|SetTargetZoom _playerpawn 5e+02))))))

(event Custom|ChangeConfigOption
  ;[1 1 1] JSON Event: Change Config Option
  (switch string (.StringValue (Class|PixelStreamingInput|GetJsonStringValue (Variables|Default|GetPixelStreamingInput) (Variables|Default|GetDescriptor) "Category"))
    (:0
      (CallFunction|ChangeCharacter))
    (:1
      (CallFunction|ChangeSkin))
    (:2
      (CallFunction|ChangeEnv))
    (:3
      (CallFunction|ChangeTime false))))

(event EventBeginPlay
  ;[1 1 1] Begin Play
  (bind _asbp_orbit_pawn (Utilities|Casting|CastToBP_Orbit_Pawn (Game|Player|GetPlayerPawn 0)))
  (Variables|Default|SetPlayerPawn _asbp_orbit_pawn)
  (bind _outactors (Actor|GetAllActorsOfClass "/Game/Blueprints/CharacterConfig/BP_CharConfig.BP_CharConfig_C"))
  (for _array_element _outactors
    (Variables|Default|SetCharConfigRef _array_element))
  (bind _outactors_2 (Actor|GetAllActorsOfClass "/Game/BP/BP_Vpa_Meta.BP_Vpa_Meta_C"))
  (for _array_element_2 _outactors_2
    (Variables|Default|SetVpaMeta _array_element_2))
  (bind _outactors_3 (Actor|GetAllActorsOfClass "/Game/BP/BP_CameraList.BP_CameraList_C"))
  (for _array_element_3 _outactors_3
    (Variables|Default|SetCameraList _array_element_3))
  ;[1 1 1] Bind JSON events - This is listening for HTM/Java events from the Pixel Streaming client's web browser.
  (EventDispatchers|BindEventtoOnInputEvent (Variables|Default|GetPixelStreamingInput) (delegate Custom|OnJSONEvent)))

(fn ConstructionScript)